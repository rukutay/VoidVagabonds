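; BP_Planet is a level planet actor with a lit body mesh and an optional instanced asteroid field.
; Its construction script applies either a custom size and texture or a random size, tilt and texture, using a dynamic material tinted by the level visual scheme's sun color.
; BeginPlay builds a circular spline and generates the asteroid field, randomizing density only after generation, or clears the instances when the field is disabled.
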(event `self.ReceiveBeginPlay`
  ; Asteroids
  (if (`self.AsteroidField`)
    (`self.BuildCircularSpline` 100.0)
    (`self.GenerateAsteroidField`)
    (set `self.DensityPer1000uu` (`KismetMathLibrary.RandomFloatInRange` 1.0 3.0))
    (else
      (`InstancedStaticMeshComponent.ClearInstances` (`self.AsteroidHISM`)))))

(event `self.ReceiveActorBeginOverlap`
  (params (OtherActor :type "Actor Object Reference")))

(fn `UserConstructionScript`
  ; CustomPlanet?
  (if (`self.Custom`)
    ; Custom Planet Size, Rotation Texture
    (`self.SetActorScale3D` (`KismetMathLibrary.Conv_DoubleToVector` (`self.CustomPlanetSize`)))
    (bind _returnvalue (`PrimitiveComponent.CreateDynamicMaterialInstance` (`self.BodyMesh`) 0 "/Game/Assets/Materials/MI_PlanetLit.MI_PlanetLit" "None"))
    (`MaterialInstanceDynamic.SetVectorParameterValue` _returnvalue "SunColor" (`LevelVisualSchemeData.SunColor` (`LevelVisualSchemeBlueprintLibrary.GetLevelVisualScheme`)))
    (`MaterialInstanceDynamic.SetTextureParameterValue` _returnvalue "PlanetTexture" (`self.CustomPlanetTexture`))
    (else
      ; Random Planet Size, Rotation, Texture
      (`self.SetActorScale3D` (`KismetMathLibrary.Conv_DoubleToVector` (`KismetMathLibrary.RandomFloatInRange` 800.0 2500.0)))
      (bind _returnvalue_2 (`PrimitiveComponent.CreateDynamicMaterialInstance` (`self.BodyMesh`) 0 "/Game/Assets/Materials/MI_PlanetLit.MI_PlanetLit" "None"))
      (`MaterialInstanceDynamic.SetVectorParameterValue` _returnvalue_2 "SunColor" (`LevelVisualSchemeData.SunColor` (`LevelVisualSchemeBlueprintLibrary.GetLevelVisualScheme`)))
      (`MaterialInstanceDynamic.SetTextureParameterValue` _returnvalue_2 "PlanetTexture" (`KismetArrayLibrary.Array_Random` (`self.PlanetTextures`)))
      (`self.K2_SetActorRotation` (`KismetMathLibrary.MakeRotator` (`KismetMathLibrary.RandomFloatInRange` 0.0 65.0) (`KismetMathLibrary.RandomFloatInRange` 0.0 65.0))))))