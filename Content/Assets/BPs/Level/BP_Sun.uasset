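; Sun actor that places a distant sun using a very long spring arm and colors it from the level visual scheme.
; It applies scheme colors to a dynamic sun material and LightColor; Custom suns also get emissive strength and a construction-time preview.
; Non-custom suns get a random scale one tick after BeginPlay.
; Construction takes emissive strength from global lighting intensity, BeginPlay from sun intensity; Tick sets ViewTargetActor to the player pawn.
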(event `self.ReceiveBeginPlay`
  (bind _returnvalue (`LevelVisualSchemeBlueprintLibrary.GetLevelVisualScheme`))
  (bind _suncolor (`LevelVisualSchemeData.SunColor` _returnvalue))
  (bind _globallightningcolor (`LevelVisualSchemeData.GlobalLightningColor` _returnvalue))
  (set `SpringArmComponent.TargetArmLength` 16000000.0 (`self.SpringArm`))
  (if (`self.Custom`)
    (bind _returnvalue_2 (`PrimitiveComponent.CreateDynamicMaterialInstance` (`self.SunMesh`) 0 "/Game/Assets/Materials/MI_Sun.MI_Sun" "None"))
    (`MaterialInstanceDynamic.SetVectorParameterValue` _returnvalue_2 "Color" _suncolor)
    (`MaterialInstanceDynamic.SetScalarParameterValue` _returnvalue_2 "EmissiveStrength" (`LevelVisualSchemeData.SunIntensity` _returnvalue))
    (set `self.LightColor` _globallightningcolor)
    (else
      (`KismetSystemLibrary.DelayUntilNextTick`)
      (`self.SetActorScale3D` (`KismetMathLibrary.Conv_DoubleToVector` (`KismetMathLibrary.RandomFloatInRange` 3500.0 6500.0)))
      (bind _returnvalue_3 (`PrimitiveComponent.CreateDynamicMaterialInstance` (`self.SunMesh`) 0 "/Game/Assets/Materials/MI_Sun.MI_Sun" "None"))
      (`MaterialInstanceDynamic.SetVectorParameterValue` _returnvalue_3 "Color" _suncolor)
      (set `self.LightColor` _globallightningcolor))))

(event `self.ReceiveTick`
  (params (DeltaSeconds :type "Float (single-precision)"))
  (set `self.ViewTargetActor` (`GameplayStatics.GetPlayerPawn` 0)))

(fn `UserConstructionScript`
  (bind _returnvalue (`LevelVisualSchemeBlueprintLibrary.GetLevelVisualScheme`))
  (if (`self.Custom`)
    (bind _returnvalue_2 (`PrimitiveComponent.CreateDynamicMaterialInstance` (`self.SunMesh`) 0 "/Game/Assets/Materials/MI_Sun.MI_Sun" "None"))
    (`MaterialInstanceDynamic.SetVectorParameterValue` _returnvalue_2 "Color" (`LevelVisualSchemeData.SunColor` _returnvalue))
    (`MaterialInstanceDynamic.SetScalarParameterValue` _returnvalue_2 "EmissiveStrength" (`LevelVisualSchemeData.GlobalLightningIntensity` _returnvalue))
    (set `self.LightColor` (`LevelVisualSchemeData.GlobalLightningColor` _returnvalue))))