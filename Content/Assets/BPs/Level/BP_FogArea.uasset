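; BP_FogArea is a level actor that creates a huge fog volume with space dust, tinted to the level's visual scheme.
; The construction script fixes the actor's scale, and BeginPlay gives the Sphere a dynamic fog material using the scheme's fog colors.
; After short tick delays, it spawns a Niagara dust system at the Collision sphere, matching its radius and the scheme's dust color.
; An older random color-scheme lookup through BP_LevelBoundaries remains disconnected.
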(event `self.ReceiveBeginPlay`
  (bind _returnvalue (`LevelVisualSchemeBlueprintLibrary.GetLevelVisualScheme`))
  (bind _collision (`self.Collision`))
  (`KismetSystemLibrary.DelayUntilNextTick`)
  (`|ExecutionSequence`
    (:`then_0`
      (`|ExecutionSequence`
        (:`then_0`
          (bind _returnvalue_2 (`PrimitiveComponent.CreateDynamicMaterialInstance` (`self.Sphere`) 0 "/Game/Assets/VFX/MI_Fog.MI_Fog" "None"))
          (`MaterialInstanceDynamic.SetVectorParameterValue` _returnvalue_2 "Albedo" (`LevelVisualSchemeData.FogColor` _returnvalue))
          (`MaterialInstanceDynamic.SetVectorParameterValue` _returnvalue_2 "Emissive" (`LevelVisualSchemeData.FogInscatteringColor` _returnvalue)))
        (:`then_1`
          (`KismetSystemLibrary.DelayUntilNextTick`)
          (bind _returnvalue_3 (`NiagaraFunctionLibrary.SpawnSystemAtLocation` "/Game/Assets/VFX/NS_SpaceDust.NS_SpaceDust" (.location (`SceneComponent.K2_GetComponentToWorld` _collision)) (.rotation (`SceneComponent.K2_GetComponentToWorld` _collision)) (1.0 1.0 1.0) false))
          (`NiagaraComponent.SetVariableFloat` _returnvalue_3 "SphereRadius" (`SphereComponent.GetScaledSphereRadius` _collision))
          (`FXSystemComponent.SetColorParameter` _returnvalue_3 "ColorMax" (`LevelVisualSchemeData.SpaceDustColorA` (`LevelVisualSchemeBlueprintLibrary.GetLevelVisualScheme`))))))))

(fn `UserConstructionScript`
  (`self.SetActorScale3D` (`KismetMathLibrary.Conv_DoubleToVector` 2000.0)))