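; BP_LevelBoundaries is a level actor with a sphere boundary, holding colour palettes and logic for populating the space inside with celestial objects.
; Its construction script fills ColorSchemas with three fog setting presets for sun, fog and dust colours.
; Unconnected graphs would spawn planets, a randomly scaled central sun and randomly scattered fog areas, passing ColorScheme to sun and fog.
; None of that spawning runs, as BeginPlay is empty.
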(event `self.ReceiveBeginPlay`)

(fn `UserConstructionScript`
  (set `self.ColorSchemas` (`|MakeArray` (make `/Game/Assets/Materials/FogSettings` (make `LinearColor` 254.0 223.0 186.0 1.0) (make `LinearColor` 216.0 216.0 216.0 1.0) (make `LinearColor` 255.0 204.0 102.0 1.0) (make `LinearColor` 255.0 170.0 90.0 1.0)) (make `/Game/Assets/Materials/FogSettings` (make `LinearColor` 255.0 100.0 200.0 1.0) (make `LinearColor` 180.0 140.0 160.0 1.0) (make `LinearColor` 255.0 170.0 220.0 1.0) (make `LinearColor` 120.0 255.0 200.0 1.0)) (make `/Game/Assets/Materials/FogSettings` (make `LinearColor` 180.0 70.0 200.0 1.0) (make `LinearColor` 140.0 130.0 255.0 1.0) (make `LinearColor` 210.0 150.0 240.0 1.0) (make `LinearColor` 120.0 255.0 230.0 1.0)))))