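; BP_ExternalModule is a ship module that automatically shoots BP_Projectile at its target actor.
; On BeginPlay it waits a tick, clears its target and derives the fire mode from its first tag, with single spelled "Simgle".
; Tick calls Shoot with speed, damage and delay when ready and the target is valid; all fire modes behave identically.
; The construction script is empty, leaving its mesh setters unconnected.
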(event `self.ReceiveBeginPlay`
  (`KismetSystemLibrary.DelayUntilNextTick`)
  (`self.ClearTarget`)
  (switch `name` (`|GetArrayItem` (`self.Tags`))
    (:`Simgle`
      (set `self.FireMode` "Single"))
    (:`Auto`
      (set `self.FireMode` "Auto"))
    (:`SemiAuto`
      (set `self.FireMode` "SemiAuto"))))

(event `self.ReceiveTick`
  (params (DeltaSeconds :type "Float (single-precision)"))
  (if (and (`self.ReadyToShoot`) (`KismetSystemLibrary.IsValid` (`self.TargetActor`)))
    (switch `EExternalModuleFireMode` (`self.FireMode`)
      (:`Single`
        _)
      (:`Auto`
        _)
      (:`SemiAuto`
        _))
    (`self.Shoot` "/Game/Assets/BPs/Ship/Module/BP_Projectile.BP_Projectile_C" (`self.ProjectileInitialSpeed`) 2.5 (`self.Damage`) (`self.ShootDelay`))))

(fn `UserConstructionScript`)