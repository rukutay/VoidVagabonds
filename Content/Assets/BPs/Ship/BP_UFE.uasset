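; BP_UFE is a ship Blueprint that sets the fire rate of its attached weapon modules when play begins.
; After the parent BeginPlay, it gathers child actor components tagged "Weapon", casts their actors to BP_ExternalModule and overrides FireRate with a fixed value.
; The construction script only calls the parent, and the Tick and overlap events are disabled.
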(event `self.ReceiveBeginPlay`
  (`parent.ReceiveBeginPlay`)
  (for _array_element (`self.GetComponentsByTag` "/Script/Engine.ChildActorComponent" "Weapon")
    (bind _asbp_external_module (cast `/Game/Assets/BPs/Ship/Module/BP_ExternalModule` (`ChildActorComponent.ChildActor` _array_element)))
    (set `ExternalModule.FireRate` 4.0 _asbp_external_module)))

(fn `UserConstructionScript`
  (`parent.UserConstructionScript`))