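; Ship actor for red-versus-blue space combat, with tagged child-actor weapon modules set to targeted turret aim.
; When attacked, it tells its AI ship controller to fight the aggressor, unless the action mode rules it out.
; SetTarget replaces an invalid target with the nearest opposite-team ship by tag and passes it to the weapons.
; Tick handles destruction with a Niagara explosion, toggles a movement effect and highlights the ship blue under the cursor.
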(event `self.ReceiveBeginPlay`
  (`SphereComponent.SetSphereRadius` (`self.InternalScanerRadius`) 6400000.0 true)
  (for _array_element (`self.GetComponentsByTag` "/Script/Engine.ChildActorComponent" "Weapon")
    (bind _asbp_external_module (cast `/Game/Assets/BPs/Ship/Module/BP_ExternalModule` (`ChildActorComponent.ChildActor` _array_element)))
    (`self.SetOwner` _asbp_external_module self)
    (set `ExternalModule.TurretAimMode` "Targeted" _asbp_external_module)))

(event `self.Attacked`
  (params (AggressorActor :type "Actor Object Reference"))
  (bind _asaiship_controller (cast `AIShipController` (`self.GetController`)))
  (if (!= (`AIShipController.ActionMode` _asaiship_controller) 4)
    (`AIShipController.Fight` _asaiship_controller AggressorActor)))

(event `self.ReceiveTick`
  (params (DeltaSeconds :type "Float (single-precision)"))
  (bind _returnvalue (`KismetMathLibrary.RandomFloatInRange` 30.0 180.0))
  (bind _shipbase (`self.ShipBase`))
  (bind (_hitresult _returnvalue_2) (`PlayerController.GetHitResultUnderCursorForObjects` (`GameplayStatics.GetPlayerController` 0) (`|MakeArray` "ObjectTypeQuery1" "ObjectTypeQuery4" "ObjectTypeQuery6" "ObjectTypeQuery8" :!type "EObjectTypeQuery Enum") false))
  (`|ExecutionSequence`
    (:`then_0`
      (if (`ShipVitalityComponent.bDestroyed` (`self.Vitality`))
        (`self.K2_DestroyActor`)
        (`NiagaraFunctionLibrary.SpawnSystemAtLocation` "/Game/Assets/VFX/NS_ShipExplosion.NS_ShipExplosion" (`self.K2_GetActorLocation`) (`KismetMathLibrary.MakeRotator` _returnvalue _returnvalue _returnvalue) (1.0 1.0 1.0) true true "None" false)))
    (:`then_1`
      (if (and (`self.isMoving`) (`self.IsPlayerLook`) (`self.isHalfSpeed`))
        (`ActorComponent.SetActive` (`self.NS_Fountain`) true false)
        (else
          (`ActorComponent.SetActive` (`self.NS_Fountain`) false true))))
    (:`then_3`
      (if (and _returnvalue_2 (== (`.HitActor` (`GameplayStatics.BreakHitResult` _hitresult)) self) (not (`self.IsPlayerLook`)))
        (`MeshComponent.SetOverlayMaterial` _shipbase "/Game/Assets/Materials/OM_Blue.OM_Blue")
        (else
          (`MeshComponent.SetOverlayMaterial` _shipbase null))))))

(fn `EvadeReset`
  (set `self.Evade?` false))

(fn `SetTarget`
  (if (not (`KismetSystemLibrary.IsValid` (`self.TargetActor`)))
    (for _array_element (`self.GetComponentsByTag` "/Script/Engine.ChildActorComponent" "Weapon")
      (bind _asbp_external_module (cast `/Game/Assets/BPs/Ship/Module/BP_ExternalModule` (`ChildActorComponent.ChildActor` _array_element)))
      (`ExternalModule.ClearTarget` _asbp_external_module))
    (switch `name` (`|GetArrayItem` (`self.Tags`))
      (:`blue`
        (bind _outactors (`GameplayStatics.GetAllActorsOfClassWithTag` "BP_Ship_C" "red"))
        (set `self.Out Actors` _outactors))
      (:`red`
        (bind _outactors_2 (`GameplayStatics.GetAllActorsOfClassWithTag` "BP_Ship_C" "blue"))
        (bind _output_get (set `self.Out Actors` _outactors_2))))
    (if (> (`KismetArrayLibrary.Array_Length` _output_get) 0)
      (bind _output_get_2 (set `self.TargetActor` (`.ReturnValue` (`GameplayStatics.FindNearestActor` (`self.K2_GetActorLocation` self) (`self.Out Actors`)))))
      (for _array_element_2 (`self.GetComponentsByTag` "/Script/Engine.ChildActorComponent" "Weapon")
        (bind _asbp_external_module_2 (cast `/Game/Assets/BPs/Ship/Module/BP_ExternalModule` (`ChildActorComponent.ChildActor` _array_element_2)))
        (`ExternalModule.SetTargetActor` _asbp_external_module_2 _output_get_2)))))

(fn `UserConstructionScript`)