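; Team-based combat ship that carries weapon modules as tagged child actors and targets ships of the opposing Red or Blue team.
; On BeginPlay it becomes the owner of each weapon module.
; Tick destroys it with a randomly rotated Niagara explosion when Vitality is destroyed, and enables target orbiting and roll alignment while its controller is in Fight mode.
; SetTarget replaces an invalid target with the nearest tagged enemy and passes it to the weapons.
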(event `self.ReceiveBeginPlay`
  (for _array_element (`self.GetComponentsByTag` "/Script/Engine.ChildActorComponent" "Weapon")
    (bind _asbp_external_module (cast `/Game/WorkElements/BPs/Ship/Module/BP_ExternalModule` (`ChildActorComponent.ChildActor` _array_element)))
    (`self.SetOwner` _asbp_external_module self)))

(event `self.ReceiveTick`
  (params (DeltaSeconds :type "Float (single-precision)"))
  (bind _returnvalue (`KismetMathLibrary.RandomFloatInRange` 30.0 180.0))
  (`|ExecutionSequence`
    (:`then_0`
      (if (`ShipVitalityComponent.bDestroyed` (`self.Vitality`))
        (`self.K2_DestroyActor`)
        (`NiagaraFunctionLibrary.SpawnSystemAtLocation` "/Game/Assets/NS_Explosion.NS_Explosion" (`self.K2_GetActorLocation`) (`KismetMathLibrary.MakeRotator` _returnvalue _returnvalue _returnvalue) (1.0 1.0 1.0) true true "None" false)))
    (:`then_1`
      (bind _asbp_ship_controller (cast `/Game/WorkElements/BPs/Controll/AI/BP_ShipController` (`self.GetController`)))
      (switch `EActionMode` (`AIShipController.ActionMode` _asbp_ship_controller)
        (:`Fight`
          (set `self.bOrbitTarget` true)
          (set `self.RollAlignMode` "BackToTarget"))))))

(fn `EvadeReset`
  (set `self.Evade?` false))

(fn `SetTarget`
  (if (not (`KismetSystemLibrary.IsValid` (`self.TargetActor`)))
    (for _array_element (`self.GetComponentsByTag` "/Script/Engine.ChildActorComponent" "Weapon")
      (bind _asbp_external_module (cast `/Game/WorkElements/BPs/Ship/Module/BP_ExternalModule` (`ChildActorComponent.ChildActor` _array_element)))
      (`ExternalModule.ClearTarget` _asbp_external_module))
    (switch `name` (`|GetArrayItem` (`self.Tags`))
      (:`blue`
        (bind _outactors (`GameplayStatics.GetAllActorsOfClassWithTag` "BP_Ship_C" "red"))
        (set `self.Out Actors` _outactors))
      (:`red`
        (bind _outactors_2 (`GameplayStatics.GetAllActorsOfClassWithTag` "BP_Ship_C" "blue"))
        (bind _output_get (set `self.Out Actors` _outactors_2))))
    (if (> (`KismetArrayLibrary.Array_Length` _output_get) 0)
      (bind _output_get_2 (set `self.TargetActor` (`.ReturnValue` (`GameplayStatics.FindNearestActor` (`self.K2_GetActorLocation` self) (`self.Out Actors`)))))
      (for _array_element_2 (`self.GetComponentsByTag` "/Script/Engine.ChildActorComponent" "Weapon")
        (bind _asbp_external_module_2 (cast `/Game/WorkElements/BPs/Ship/Module/BP_ExternalModule` (`ChildActorComponent.ChildActor` _array_element_2)))
        (`ExternalModule.SetTargetActor` _asbp_external_module_2 _output_get_2)))))

(fn `UserConstructionScript`)