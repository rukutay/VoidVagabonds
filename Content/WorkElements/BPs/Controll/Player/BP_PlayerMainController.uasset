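; BP_PlayerMainController is the player controller for viewing, possessing and selecting ships.
; On BeginPlay and on Z it calls LookAtActor on a random BP_Ship tagged "player", while X passes a random one to SwitchToPawn.
; Left click traces under the cursor against selected object types and sets FocusActor to a hit actor with a MarkerComponent, otherwise clears it.
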(event `self.ReceiveBeginPlay`
  (bind _outactors (`GameplayStatics.GetAllActorsOfClassWithTag` "/Game/WorkElements/BPs/Ship/BP_Ship.BP_Ship_C" "player"))
  (`self.LookAtActor` (`KismetArrayLibrary.Array_Random` _outactors)))

(event `Key|X`
  (params (Key :type "Key Structure"))
  (:`Pressed`
    (bind _outactors (`GameplayStatics.GetAllActorsOfClassWithTag` "/Game/WorkElements/BPs/Ship/BP_Ship.BP_Ship_C" "player"))
    (`self.SwitchToPawn` (`KismetArrayLibrary.Array_Random` _outactors))))

(event `Key|Z`
  (params (Key :type "Key Structure"))
  (:`Pressed`
    (bind _outactors (`GameplayStatics.GetAllActorsOfClassWithTag` "/Game/WorkElements/BPs/Ship/BP_Ship.BP_Ship_C" "player"))
    (`self.LookAtActor` (`KismetArrayLibrary.Array_Random` _outactors))))

(event `Key|LeftMouseButton`
  (params (Key :type "Key Structure"))
  (bind (_hitresult _returnvalue) (`self.GetHitResultUnderCursorForObjects` (`|MakeArray` "ObjectTypeQuery1" "ObjectTypeQuery4" "ObjectTypeQuery6" "ObjectTypeQuery8" :!type "EObjectTypeQuery Enum") false))
  (bind (_bblockinghit _binitialoverlap _time _distance _location _impactpoint _normal _impactnormal _physmat _hitactor) (`GameplayStatics.BreakHitResult` _hitresult))
  (:`Pressed`
    (if (and _returnvalue (`KismetSystemLibrary.IsValid` (`self.GetComponentByClass` _hitactor "/Script/VagabondsWork.MarkerComponent")))
      (set `self.FocusActor` _hitactor)
      (else
        (set `self.FocusActor` null)))))

(fn `UserConstructionScript`)