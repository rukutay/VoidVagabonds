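; Level boundary actor that procedurally populates a space level with a sun, planets and fog at BeginPlay.
; After a one-tick delay it picks a random color palette from those built in the construction script and spawns a randomly scaled sun at its location.
; NavStaticBig handles planet placement, then FogSpawn scatters palette-tinted fog spheres around world origin, between a minimum distance and the Boudaries sphere radius.
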(event `self.ReceiveBeginPlay`
  (`KismetSystemLibrary.DelayUntilNextTick`)
  (`|ExecutionSequence`
    (:`then_0`
      (set `self.ColorScheme` (`KismetArrayLibrary.Array_Random` (`self.ColorSchemas`))))
    (:`then_1`
      (bind _returnvalue (`|SpawnActorFromClass` "/Game/WorkElements/BPs/Level/BP_Sun.BP_Sun_C" (`KismetMathLibrary.MakeTransform` (`self.K2_GetActorLocation`) (struct) (`KismetMathLibrary.Conv_DoubleToVector` (`KismetMathLibrary.RandomFloatInRange` 1500.0 3500.0))) "AlwaysSpawn" "MultiplyWithRoot" null 0 null))
      (set `/Game/WorkElements/BPs/Level/BP_Sun.ColorScheme` (`self.ColorScheme`) _returnvalue))
    (:`then_2`
      (`self.NavStaticBig` "/Game/WorkElements/BPs/Level/BP_Planet.BP_Planet_C" 1 4 1000000.0))
    (:`then_3`
      (for _ (range (+ (`KismetMathLibrary.FTrunc` (`KismetMathLibrary.RandomFloatInRange` 1.0 100.0)) 1))
        (bind _returnvalue_2 (`|SpawnActorFromClass` "/Game/WorkElements/BPs/Level/BP_FogSphere.BP_FogSphere_C" (`KismetMathLibrary.MakeTransform` (* (`KismetMathLibrary.RandomUnitVector`) (`KismetMathLibrary.RandomFloatInRange` 250000.0 (`SphereComponent.GetScaledSphereRadius` (`self.Boudaries`))))) "AlwaysSpawn" "MultiplyWithRoot" self null))
        (set `/Game/WorkElements/BPs/Level/BP_FogSphere.ColorScheme` (`self.ColorScheme`) _returnvalue_2)))))

(fn `UserConstructionScript`
  (set `self.ColorSchemas` (`|MakeArray` (make `/Game/Assets/Materials/FogSettings` (make `LinearColor` 59.0 151.0 151.0 1.0) (make `LinearColor` 19.0 36.0 64.0 1.0) (make `LinearColor` 22.0 71.0 106.0 1.0) (make `LinearColor` 191.0 9.0 47.0 1.0)) (make `/Game/Assets/Materials/FogSettings` (make `LinearColor` 220.0 0.0 0.0 1.0) (make `LinearColor` 5.0 14.0 60.0 1.0) (make `LinearColor` 0.0 36.0 85.0 1.0) (make `LinearColor` 255.0 56.0 56.0 1.0)) (make `/Game/Assets/Materials/FogSettings` (make `LinearColor` 244.0 179.0 66.0 1.0) (make `LinearColor` 143.0 1.0 119.0 1.0) (make `LinearColor` 222.0 26.0 88.0 1.0) (make `LinearColor` 54.0 1.0 133.0 1.0)))))