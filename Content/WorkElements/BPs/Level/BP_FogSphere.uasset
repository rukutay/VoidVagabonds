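; BP_FogSphere is a huge fog volume, scaled up in the construction script, that adds colored fog and space dust to the level.
; On BeginPlay it picks a random color scheme from its owning BP_LevelBoundaries, or from one found in the level if it has no owner.
; The scheme tints a dynamic fog material on the sphere and a SpaceDust2 Niagara system spawned to match the collision radius.
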(event `self.ReceiveBeginPlay`
  (bind _returnvalue (`self.GetOwner`))
  (bind _collision (`self.Collision`))
  (bind (_colorscheme_suncolor _colorscheme_fogbase _colorscheme_fogemissive _colorscheme_dust) (break `/Game/Assets/Meshes/Materials/FogSettings` (`self.ColorScheme`)))
  (bind (_colorscheme_suncolor_2 _colorscheme_fogbase_2 _colorscheme_fogemissive_2 _colorscheme_dust_2) (break `/Game/Assets/Meshes/Materials/FogSettings` (`self.ColorScheme`)))
  (`KismetSystemLibrary.DelayUntilNextTick`)
  (`|ExecutionSequence`
    (:`then_0`
      (if (`KismetSystemLibrary.IsValid` _returnvalue)
        (bind _asbp_level_boundaries (cast `/Game/WorkElements/BPs/Level/BP_LevelBoundaries` _returnvalue))
        (set `self.ColorScheme` (`KismetArrayLibrary.Array_Random` (`/Game/WorkElements/BPs/Level/BP_LevelBoundaries.ColorSchemas` _asbp_level_boundaries)))
        (else
          (bind _returnvalue_2 (`GameplayStatics.GetActorOfClass` "/Game/WorkElements/BPs/Level/BP_LevelBoundaries.BP_LevelBoundaries_C"))
          (set `self.ColorScheme` (`KismetArrayLibrary.Array_Random` (`/Game/WorkElements/BPs/Level/BP_LevelBoundaries.ColorSchemas` _returnvalue_2))))))
    (:`then_1`
      (`|ExecutionSequence`
        (:`then_0`
          (bind _returnvalue_3 (`PrimitiveComponent.CreateDynamicMaterialInstance` (`self.Sphere`) 0 "/Game/Assets/Meshes/Materials/VFX/MM_Fog1_Inst.MM_Fog1_Inst" "None"))
          (`MaterialInstanceDynamic.SetVectorParameterValue` _returnvalue_3 "Albedo" _colorscheme_fogbase)
          (`MaterialInstanceDynamic.SetVectorParameterValue` _returnvalue_3 "Emissive" (/ _colorscheme_dust 100000.0)))
        (:`then_1`
          (`KismetSystemLibrary.DelayUntilNextTick`)
          (bind _returnvalue_4 (`NiagaraFunctionLibrary.SpawnSystemAtLocation` "/Game/Assets/Meshes/Materials/VFX/SpaceDust2.SpaceDust2" (.location (`SceneComponent.K2_GetComponentToWorld` _collision)) (.rotation (`SceneComponent.K2_GetComponentToWorld` _collision)) (1.0 1.0 1.0) false))
          (`NiagaraComponent.SetVariableFloat` _returnvalue_4 "SphereRadius" (`SphereComponent.GetScaledSphereRadius` _collision))
          (`FXSystemComponent.SetColorParameter` _returnvalue_4 "ColorMax" _colorscheme_dust_2))))))

(fn `UserConstructionScript`
  (`self.SetActorScale3D` (`KismetMathLibrary.Conv_DoubleToVector` 2000.0)))