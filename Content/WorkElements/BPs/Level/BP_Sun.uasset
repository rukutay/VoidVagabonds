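; BP_Sun is a level sun actor whose color comes from the color scheme.
; One tick after BeginPlay it creates a dynamic MI_Sun material on the sun mesh, applies the scaled-down scheme color to it and to LightColor, and multiplies the spring arm length by actor X scale.
; Every tick it sets ViewTargetActor to the first player's pawn.
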(event `self.ReceiveBeginPlay`
  (bind _colorscheme_suncolor (break `/Game/Assets/Materials/FogSettings` (`self.ColorScheme`)))
  (bind _springarm (`self.SpringArm`))
  (bind _returnvalue (/ _colorscheme_suncolor 1000.0))
  (bind _returnvalue_x (`KismetMathLibrary.BreakVector` (* (`self.GetActorScale3D`) (`SpringArmComponent.TargetArmLength` _springarm))))
  (`KismetSystemLibrary.DelayUntilNextTick`)
  (bind _returnvalue_2 (`PrimitiveComponent.CreateDynamicMaterialInstance` (`self.SunMesh`) 0 "/Game/Assets/Materials/MI_Sun.MI_Sun" "None"))
  (`MaterialInstanceDynamic.SetVectorParameterValue` _returnvalue_2 "Color" _returnvalue)
  (set `self.LightColor` _returnvalue)
  (set `SpringArmComponent.TargetArmLength` _returnvalue_x _springarm))

(event `self.ReceiveTick`
  (params (DeltaSeconds :type "Float (single-precision)"))
  (set `self.ViewTargetActor` (`GameplayStatics.GetPlayerPawn` 0)))

(fn `UserConstructionScript`)