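; BP_Planet is a level actor that forms a randomized planet, sometimes circled by an asteroid field.
; The construction script randomizes its scale, and BeginPlay randomizes its tilt.
; One tick later, a coin flip decides whether to build a circular spline and asteroid field, setting a random density only after generation.
; A dynamic material on the body gets a random planet texture and BP_Sun's color.
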(event `self.ReceiveBeginPlay`
  (`self.K2_SetActorRotation` (`KismetMathLibrary.MakeRotator` (`KismetMathLibrary.RandomFloatInRange` 0.0 65.0) (`KismetMathLibrary.RandomFloatInRange` 0.0 65.0)))
  (`KismetSystemLibrary.DelayUntilNextTick`)
  (if (`KismetMathLibrary.RandomBool`)
    (`self.BuildCircularSpline` 100.0)
    (`self.GenerateAsteroidField`)
    (set `self.DensityPer1000uu` (`KismetMathLibrary.RandomFloatInRange` 2.0 5.0)))
  (bind _returnvalue (`GameplayStatics.GetActorOfClass` "/Game/WorkElements/BPs/Level/BP_Sun.BP_Sun_C"))
  (bind _returnvalue_2 (`PrimitiveComponent.CreateDynamicMaterialInstance` (`self.BodyMesh`) 0 "/Game/Assets/Materials/MI_PlanetLit.MI_PlanetLit" "None"))
  (`MaterialInstanceDynamic.SetVectorParameterValue` _returnvalue_2 "SunColor" (`.SunColor_14_7A44FA76928441B4822AB8AECA3AACF7` (break `/Game/Assets/Materials/FogSettings` (`/Game/WorkElements/BPs/Level/BP_Sun.ColorScheme` _returnvalue))))
  (`MaterialInstanceDynamic.SetTextureParameterValue` _returnvalue_2 "PlanetTexture" (`KismetArrayLibrary.Array_Random` (`self.PlanetTextures`))))

(event `self.ReceiveActorBeginOverlap`
  (params (OtherActor :type "Actor Object Reference")))

(fn `UserConstructionScript`
  (`self.SetActorScale3D` (`KismetMathLibrary.Conv_DoubleToVector` (`KismetMathLibrary.RandomFloatInRange` 700.0 1800.0))))